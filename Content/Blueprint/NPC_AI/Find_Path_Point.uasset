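; Behavior tree task that picks the patrol destination for an EnemyCharacter.
; It reads the path index from the blackboard, converts that PatrolPath point from the path actor's local space to world space, and writes it to the path vector key.
; It finishes successfully only when the patrol path is valid; a failed cast or missing path never calls FinishExecute.
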(event `self.ReceiveExecuteAI`
  (params (OwnerController :type "AIController Object Reference") (ControlledPawn :type "Pawn Object Reference"))
  (bind _asenemy_character (cast `/Game/Blueprint/NPC_AI/EnemyCharacter` ControlledPawn))
  (bind _patrolpath (`/Game/Blueprint/NPC_AI/EnemyCharacter.PatrolPath` _asenemy_character)
    (:`then`
      (`BTFunctionLibrary.SetBlackboardValueAsVector` (`self.BB_PathVector`) (`KismetMathLibrary.TransformLocation` (`Actor.GetTransform` _patrolpath) (`|GetArrayItem` (`/Game/Blueprint/NPC_AI/ControllPath.PathPoints` _patrolpath) (`BTFunctionLibrary.GetBlackboardValueAsInt` (`self.BB_PathIndex`)))))
      (`self.FinishExecute` true))
    (:`else`)))