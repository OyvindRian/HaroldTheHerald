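; Behavior Tree task that advances an enemy NPC's patrol index forward along its path.
; When the blackboard direction is 1, it checks the next index against the EnemyCharacter's PatrolPath points, then increments it and succeeds.
; At the last point it flips the direction to -1 and fails, as it does for any other direction.
; A failed pawn cast leaves the task unfinished.
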(event `self.ReceiveExecuteAI`
  (params (OwnerController :type "AIController Object Reference") (ControlledPawn :type "Pawn Object Reference"))
  (bind _bb_direction (`self.BB_Direction`))
  (bind _returnvalue (+ (`BTFunctionLibrary.GetBlackboardValueAsInt` (`self.BB_PathIndex`)) 1))
  (if (== (`BTFunctionLibrary.GetBlackboardValueAsInt` (`self.BB_Direction`)) 1)
    (bind _asenemy_character (cast `/Game/Blueprint/NPC_AI/EnemyCharacter` ControlledPawn))
    (if (<= _returnvalue (- (`KismetArrayLibrary.Array_Length` (`/Game/Blueprint/NPC_AI/ControllPath.PathPoints` (`/Game/Blueprint/NPC_AI/EnemyCharacter.PatrolPath` _asenemy_character))) 1))
      (`BTFunctionLibrary.SetBlackboardValueAsInt` _bb_direction 1)
      (`BTFunctionLibrary.SetBlackboardValueAsInt` (`self.BB_PathIndex`) _returnvalue)
      (`self.FinishExecute` true)
      (else
        (`BTFunctionLibrary.SetBlackboardValueAsInt` _bb_direction -1)
        (`self.FinishExecute` false)))
    (else
      (`self.FinishExecute` false))))