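; Skeleton enemy character, labeled unused, that damages the twin-stick player on overlap and loses health from amplified radial damage or DamageHealth.
; A delayed Tick check calls EnemyDeath at a health threshold, destroying it with explosion effects and a 50% chance to spawn Skeleton_spawn.
; Construction tints the body red through a dynamic material.
; A separate EnemyDamage function applies force and destroys below zero health, while health bar updating is disconnected.
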(event `self.ReceiveRadialDamage`
  (params (DamageReceived :type "Float (single-precision)") (DamageType :type "DamageType Object Reference") (Origin :type "Vector Structure") (HitInfo :type "HitResult Structure (by ref)") (InstigatedBy :type "Controller Object Reference") (DamageCauser :type "Actor Object Reference"))
  ;[1 1 1] UNUSED CHARACTER
  ;;[1 1 1] Take Radial Damage
  (bind _output_get (set `self.Health_0` (- (`self.Health_0`) (* DamageReceived 5.0)))))

(event `ExplodingEnemyTrigger`
  ;[1 1 1] UNUSED CHARACTER
)

(event `self.ReceiveTick`
  (params (DeltaSeconds :type "Float (single-precision)"))
  ;[1 1 1] UNUSED CHARACTER
  ;;[1 1 1] Event Tick
  (`|ExecutionSequence`
    (:`then_0`
      ;;[1 1 1] Check For Actor Death
      (`KismetSystemLibrary.Delay` 0.2)
      (if (<= (`self.Health_0`) 100.0)
        (`self.EnemyDeath`)))
    (:`then_1`
      (`self.UpdateHealthBar`))))

(event `UpdateHealthBar`
  ;[1 1 1] UNUSED CHARACTER
  ;;[1 1 1] Update Health Bar
)

(event `self.ReceiveActorBeginOverlap`
  (params (OtherActor :type "Actor Object Reference"))
  ;[1 1 1] UNUSED CHARACTER
  ;;[1 1 1] Damage Player
  (bind _asbp_twin_stick_character (cast `/Game/Blueprint/BP_TwinStickCharacter` OtherActor))
  (`/Game/Blueprint/BP_TwinStickCharacter.DamagePlayer` _asbp_twin_stick_character))

(event `EnemyDeath`
  (bind _returnvalue (`self.K2_GetActorLocation`))
  ;[1 1 1] UNUSED CHARACTER
  ;;[1 1 1] Spawn Sound, Effect and Bones (50% chance)
  (`self.K2_DestroyActor`)
  (`GameplayStatics.PlaySoundAtLocation` "/Game/sound/SC_MissileExplosion.SC_MissileExplosion")
  (`GameplayStatics.SpawnEmitterAtLocation` "/Game/VFX_Toolkit_V1/ParticleSystems/356Days/Par_ToonKaboom_01.Par_ToonKaboom_01" _returnvalue (struct) (0.45 0.45 0.45))
  (`GameplayStatics.SpawnEmitterAtLocation` "/Game/VFX_Toolkit_V1/ParticleSystems/356Days/Par_BombWaker.Par_BombWaker" _returnvalue (struct) (0.3 0.4 0.4))
  (if (`KismetMathLibrary.RandomBoolWithWeight` 0.5)
    (`|SpawnActorFromClass` "/Game/Blueprint/skeleton_spawn.skeleton_spawn_C" (`self.GetTransform`) "Undefined" "OverrideRootScale" null null)))

(event `DamageHealth`
  ;[1 1 1] UNUSED CHARACTER
  ;;[1 1 1] Enemy Take Damage
  (set `self.Health_0` (- (`self.Health_0`) (`self.DamageAmount`))))

(fn `Enemy Damage`
  (set `self.Health_0` (`self.Health_0`))
  (`CharacterMovementComponent.AddForce` (`self.CharacterMovement`) (+ (* (`self.K2_GetActorLocation`) -5000) (`self.GetActorForwardVector`)))
  (if (< (`self.Health_0`) 0.0)
    (`self.K2_DestroyActor`)))

(fn `UserConstructionScript`
  (bind _returnvalue (`PrimitiveComponent.CreateDynamicMaterialInstance` (`self.Mesh`) 0 null))
  (bind _output_get (set `self.DynoMat` _returnvalue))
  (`MaterialInstanceDynamic.SetVectorParameterValue` _output_get "BodyColor" (struct :`R` 1.0 :`G` 0.009844 :`A` 1.0)))