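; Weapon actor that fires Laser projectiles from a spawn point with sound, muzzle flash and camera shake.
; PullTrigger waits a short fire-rate delay, then calls Fire, which spawns the laser and attaches an explosion sound to the skeletal mesh.
; Fire also shakes the first player's camera and briefly pulses the muzzle flash, which BeginPlay switches off at start.
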(event `Pull Trigger`
  ;[1 1 1] FireRate
  (`KismetSystemLibrary.Delay` 0.12)
  (`self.Fire`))

(event `Fire`
  (bind _muzzleflash (`self.MuzzleFlash`))
  (`GameplayStatics.SpawnSoundAttached` "/Game/sound/SC_MissileExplosion.SC_MissileExplosion" (`self.SkeletalMesh`) "None" (0.0 0.0 0.0) (struct) "KeepRelativeOffset" false 4.0 0.5 1.0)
  ;[1 1 1] Spawn Lasor on Spawn Point
  (`|SpawnActorFromClass` "/Game/Blueprint/Laser.Laser_C" (`SceneComponent.K2_GetComponentToWorld` (`self.ProjectileSpawnPoint`)) "Undefined" "OverrideRootScale" null null)
  (`PlayerController.ClientStartCameraShake` :`self` (`GameplayStatics.GetPlayerController` 0) :`Shake` "/Game/Blueprint/CameraShakeWeapon.CameraShakeWeapon_C" :`Scale` 0.1)
  ;[1 1 1] "Muzzle Flash"
  (`ActorComponent.Activate` _muzzleflash false)
  (`KismetSystemLibrary.Delay` 0.01)
  (`ActorComponent.Deactivate` _muzzleflash))

(event `self.ReceiveBeginPlay`
  ;[1 1 1] "Muzzle Flash"
  (`ActorComponent.Deactivate` (`self.MuzzleFlash`)))

(fn `UserConstructionScript`)