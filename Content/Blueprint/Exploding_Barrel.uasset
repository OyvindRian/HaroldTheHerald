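; Explosive barrel that loses health from Laser overlaps or general damage and blows up.
; A laser hit leaving health at or below a threshold activates its particle effect and starts a delayed blast with layered effects, camera shake and a spawned Explosion actor.
; Radial damage skips that fuse for a similar blast.
; Tick checks for zero health, cutting the fuse short with a simpler EnemyDeath effect that spawns no Explosion actor.
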(event `self.ReceiveAnyDamage`
  (params (Damage :type "Float (single-precision)") (DamageType :type "DamageType Object Reference") (InstigatedBy :type "Controller Object Reference") (DamageCauser :type "Actor Object Reference"))
  ;[1 1 1] test
  (set `self.Health` (- (`self.Health`) Damage)))

(event `DamageHealth`
  ;[1 1 1] Test
  (set `self.Health` (- (`self.Health`) (`self.DamageAmount`))))

(event `self.ReceiveTick`
  (params (DeltaSeconds :type "Float (single-precision)"))
  ;[1 1 1] Event Tick
  ;[1 1 1] Check For Actor Death
  (if (<= (`self.Health`) 0.0)
    (`self.EnemyDeath`)))

(event `EnemyDeath`
  ;[1 1 1] Explode Before the timer runs out because player shot it enough
  (`GameplayStatics.PlaySoundAtLocation` "/Game/sound/Explosion_Cue.Explosion_Cue")
  (`GameplayStatics.SpawnEmitterAtLocation` "/Game/VFX_Toolkit_V1/ParticleSystems/356Days/Par_Meteora_Explode_01.Par_Meteora_Explode_01" (`self.K2_GetActorLocation`))
  (`self.K2_DestroyActor`))

(event `self.collision.OnComponentBeginOverlap`
  (params (OverlappedComponent :type "PrimitiveComponent Object Reference") (OtherActor :type "Actor Object Reference") (OtherComp :type "PrimitiveComponent Object Reference") (OtherBodyIndex :type Integer) (bFromSweep :type Boolean) (SweepResult :type "HitResult Structure (by ref)"))
  (bind _returnvalue (`SceneComponent.K2_GetComponentLocation` (`self.Barrel`)))
  ;[1 1 1] Check for health.  if health <= 150 == explode in 1.5. IF Health == 0, Explode before time runs out
  (cast `/Game/Blueprint/Laser` OtherActor)
  (set `self.Health` (- (`self.Health`) (`self.DamageAmount`)))
  (if (<= (`self.Health`) 150.0)
    ;[1 1 1] Explode when shot + sound and effetcs
    (`ActorComponent.Activate` (`self.ParticleSystem`) false)
    ;;[1 1 1] Explode in 1.5 sec
    (`KismetSystemLibrary.Delay` 1.5)
    (`GameplayStatics.SpawnEmitterAtLocation` "/Game/VFX_Toolkit_V1/ParticleSystems/356Days/Par_MatraBoom_01.Par_MatraBoom_01" _returnvalue (`KismetMathLibrary.Conv_VectorToRotator` _returnvalue) (2.0 2.0 2.0))
    (`GameplayStatics.SpawnSoundAtLocation` "/Game/sound/SC_MissileExplosion.SC_MissileExplosion" _returnvalue (`KismetMathLibrary.Conv_VectorToRotator` _returnvalue) 10.0 0.5)
    (`KismetSystemLibrary.Delay` 0.2)
    (`GameplayStatics.SpawnEmitterAtLocation` "/Game/VFX_Toolkit_V1/ParticleSystems/356Days/Par_MatraBoom_01.Par_MatraBoom_01" _returnvalue (`KismetMathLibrary.Conv_VectorToRotator` _returnvalue) (5.0 5.0 5.0))
    (`GameplayStatics.SpawnEmitterAtLocation` "/Game/VFX_Toolkit_V1/ParticleSystems/356Days/Par_Meteora_Explode_01.Par_Meteora_Explode_01" _returnvalue (`KismetMathLibrary.Conv_VectorToRotator` _returnvalue))
    ;;[1 1 1] Spawn Explosion Bp
    (`PlayerController.ClientStartCameraShake` :`self` (`GameplayStatics.GetPlayerController` 0) :`Shake` "/Game/Blueprint/CameraShakeWeapon.CameraShakeWeapon_C" :`Scale` 0.5)
    (`|SpawnActorFromClass` "/Game/Blueprint/Explosion.Explosion_C" (`KismetMathLibrary.Conv_VectorToTransform` (`SceneComponent.K2_GetComponentLocation` (`self.Barrel`))) "Undefined" "OverrideRootScale" null null)
    (`PlayerController.ClientStartCameraShake` :`self` (`GameplayStatics.GetPlayerController` 0) :`Shake` "/Game/Blueprint/CameraShakeWeapon.CameraShakeWeapon_C" :`Scale` 1.2)
    (`self.K2_DestroyActor`)
    (elif (<= (`self.Health`) 0.0)
      (`self.EnemyDeath`))))

(event `self.ReceiveBeginPlay`
  ;[1 1 1] Explode when shot + sound and effetcs
  (`ActorComponent.Deactivate` (`self.ParticleSystem`)))

(event `self.ReceiveRadialDamage`
  (params (DamageReceived :type "Float (single-precision)") (DamageType :type "DamageType Object Reference") (Origin :type "Vector Structure") (HitInfo :type "HitResult Structure (by ref)") (InstigatedBy :type "Controller Object Reference") (DamageCauser :type "Actor Object Reference"))
  (bind _returnvalue (`SceneComponent.K2_GetComponentLocation` (`self.Barrel`)))
  ;[1 1 1] Instantly Explode on Radial Damage
  (`GameplayStatics.SpawnEmitterAtLocation` "/Game/VFX_Toolkit_V1/ParticleSystems/356Days/Par_MatraBoom_01.Par_MatraBoom_01" _returnvalue (`KismetMathLibrary.Conv_VectorToRotator` _returnvalue) (2.0 2.0 2.0))
  (`GameplayStatics.SpawnSoundAtLocation` "/Game/sound/SC_MissileExplosion.SC_MissileExplosion" _returnvalue (`KismetMathLibrary.Conv_VectorToRotator` _returnvalue) 10.0 0.5)
  (`KismetSystemLibrary.Delay` 0.2)
  (`GameplayStatics.SpawnEmitterAtLocation` "/Game/VFX_Toolkit_V1/ParticleSystems/356Days/Par_MatraBoom_01.Par_MatraBoom_01" _returnvalue (`KismetMathLibrary.Conv_VectorToRotator` _returnvalue) (5.0 5.0 5.0))
  (`GameplayStatics.SpawnEmitterAtLocation` "/Game/VFX_Toolkit_V1/ParticleSystems/356Days/Par_Meteora_Explode_01.Par_Meteora_Explode_01" _returnvalue (`KismetMathLibrary.Conv_VectorToRotator` _returnvalue))
  (`PlayerController.ClientStartCameraShake` :`self` (`GameplayStatics.GetPlayerController` 0) :`Shake` "/Game/Blueprint/CameraShakeWeapon.CameraShakeWeapon_C" :`Scale` 0.5)
  (`|SpawnActorFromClass` "/Game/Blueprint/Explosion.Explosion_C" (`KismetMathLibrary.Conv_VectorToTransform` (`SceneComponent.K2_GetComponentLocation` (`self.Fire`))) "Undefined" "OverrideRootScale" null null)
  (`PlayerController.ClientStartCameraShake` :`self` (`GameplayStatics.GetPlayerController` 0) :`Shake` "/Game/Blueprint/CameraShakeWeapon.CameraShakeWeapon_C" :`Scale` 1.2)
  (`self.K2_DestroyActor`))

(fn `UserConstructionScript`)