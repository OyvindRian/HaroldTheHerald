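; Enemy spawner that, each time SpawnEnemy is called, can release a staggered group of normal, goblin and exploding enemies until its horde budget runs out.
; A live-count check on either normal or exploding enemies being under its cap triggers the shared delayed spawn chain, which decrements the budget.
; Each enemy spawns at a random point inside the SpawnVolum box.
; A DoOnce plays a sound at the spawner on first activation.
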(event `SpawnEnemy`
  (bind _spawnvolum (`self.SpawnVolum`))
  (bind _returnvalue (`KismetMathLibrary.RandomPointInBoundingBox` (`SceneComponent.K2_GetComponentLocation` _spawnvolum) (`BoxComponent.GetScaledBoxExtent` _spawnvolum)))
  (if (>= (`self.Max Spawned Enemies`) 0.0)
    (`|ExecutionSequence`
      (:`then_0`
        (bind _outactors (`GameplayStatics.GetAllActorsOfClass` "/Game/Blueprint/NPC_AI/EnemyCharacter.EnemyCharacter_C"))
        (if (< (`KismetArrayLibrary.Array_Length` _outactors) (`self.Max enemies`))
          (`KismetSystemLibrary.Delay` 0.7 :!label _label)
          (bind _result (`/Engine/EditorBlueprintResources/StandardMacros.DecrementFloat` (`self.Max Spawned Enemies`))
            (:`  `
              (set `self.Max Spawned Enemies` _result)
              ;[1 1 1] Spawn Enemies in "Rarity" Normal, goblin, exploding enemy
              (`AIBlueprintHelperLibrary.SpawnAIFromClass` "/Game/Blueprint/NPC_AI/EnemyCharacter.EnemyCharacter_C" null _returnvalue)
              (`KismetSystemLibrary.Delay` 0.5)
              (`AIBlueprintHelperLibrary.SpawnAIFromClass` "/Game/Blueprint/BP_Goblin.BP_Goblin_C" null _returnvalue)
              (`KismetSystemLibrary.Delay` 3.0)
              (`AIBlueprintHelperLibrary.SpawnAIFromClass` "/Game/Blueprint/Exploding_enemy.Exploding_enemy_C" null _returnvalue)))))
      (:`then_1`
        (bind _outactors_2 (`GameplayStatics.GetAllActorsOfClass` "/Game/Blueprint/Exploding_enemy.Exploding_enemy_C"))
        (if (< (`KismetArrayLibrary.Array_Length` _outactors_2) (`self.Max Exploding Enemy`))
          (goto _label)))
      (:`then_2`
        (`/Engine/EditorBlueprintResources/StandardMacros.DoOnce` false
          (:`Completed`
            (`GameplayStatics.PlaySoundAtLocation` "/Game/sound/Waaagh-jt_9fsA_XmA.Waaagh-jt_9fsA_XmA" (`self.K2_GetActorLocation`) (struct) 0.5 0.8)))))))

(fn `UserConstructionScript`)