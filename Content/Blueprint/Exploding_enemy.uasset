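; Exploding enemy character that, on death, ignites and speeds up as a running bomb before blowing up.
; EnemyDeath activates the fire particles, then either explodes immediately if health is far below zero or starts a short fuse.
; Radial damage also triggers instant detonation.
; Detonation staggers small and full-size emitters, deals radial damage, plays a sound and destroys the actor.
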(event `self.ReceiveRadialDamage`
  (params (DamageReceived :type "Float (single-precision)") (DamageType :type "DamageType Object Reference") (Origin :type "Vector Structure") (HitInfo :type "HitResult Structure (by ref)") (InstigatedBy :type "Controller Object Reference") (DamageCauser :type "Actor Object Reference"))
  (bind _returnvalue (`self.K2_GetActorLocation`))
  ;[1 1 1] Instanly explode when taking radial damage
  (`GameplayStatics.SpawnEmitterAtLocation` "/Game/VFX_Toolkit_V1/ParticleSystems/356Days/Par_Meteora_Explode_01.Par_Meteora_Explode_01" _returnvalue (struct) (0.5 0.5 0.5) :!label _label)
  (`KismetSystemLibrary.Delay` 0.2)
  (`GameplayStatics.SpawnEmitterAtLocation` "/Game/VFX_Toolkit_V1/ParticleSystems/356Days/Par_Meteora_Explode_01.Par_Meteora_Explode_01" _returnvalue)
  (`GameplayStatics.ApplyRadialDamage` :`BaseDamage` 20.0 :`Origin` _returnvalue :`DamageRadius` 400.0 :`DamageCauser` self :`InstigatedByController` (`self.GetInstigatorController`) :`bDoFullDamage` true)
  (`GameplayStatics.PlaySoundAtLocation` "/Game/sound/Explosion_Cue.Explosion_Cue" (`self.K2_GetActorLocation`) (struct) 1.2)
  (`self.K2_DestroyActor`))

(event `self.ReceiveBeginPlay`
  ;[1 1 1] Deactivate fire effect
  (`ActorComponent.Deactivate` (`self.ParticleSystem`)))

(event `Explode`
  ;[1 1 1] Explode Before timer runs out Because player shot him enough
  (goto _label))

(event `self.EnemyDeath`
  ;[1 1 1] "Active" Running Exploding Man
  (`ActorComponent.Activate` (`self.ParticleSystem`) false)
  (set `CharacterMovementComponent.MaxWalkSpeed` 800.0 (`self.CharacterMovement`))
  (if (<= (`self.Health_0`) -50.0)
    (`self.Explode`)
    (else
      (`self.Running exploding_Enemy`))))

(event `Running exploding_Enemy`
  (bind _returnvalue (`self.K2_GetActorLocation`))
  ;[1 1 1] Stop movement when "dead". Explode after 1 second
  (`KismetSystemLibrary.Delay` 1.0)
  (`GameplayStatics.SpawnEmitterAtLocation` "/Game/VFX_Toolkit_V1/ParticleSystems/356Days/Par_Meteora_Explode_01.Par_Meteora_Explode_01" _returnvalue (struct) (0.5 0.5 0.5))
  (`KismetSystemLibrary.Delay` 0.2)
  (`GameplayStatics.SpawnEmitterAtLocation` "/Game/VFX_Toolkit_V1/ParticleSystems/356Days/Par_Meteora_Explode_01.Par_Meteora_Explode_01" _returnvalue)
  (`GameplayStatics.ApplyRadialDamage` :`BaseDamage` 20.0 :`Origin` _returnvalue :`DamageRadius` 400.0 :`DamageCauser` self :`InstigatedByController` (`self.GetInstigatorController`) :`bDoFullDamage` true)
  (`GameplayStatics.PlaySoundAtLocation` "/Game/sound/Explosion_Cue.Explosion_Cue" (`self.K2_GetActorLocation`) (struct) 1.2)
  (`self.K2_DestroyActor`))

(fn `UserConstructionScript`
  (`parent.UserConstructionScript`))