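; Laser projectile actor that damages what it touches, playing an explosion sound and destroying itself on impact.
; On overlap, it sends Damage through the IDamageable interface, ignores damageable actors tagged Friendly, and also explodes on non-damageable actors.
; After exploding, it additionally calls DamageHealth on EnemyCharacter targets.
; A separate Hit handler destroys the other actor, then calls DamageHealth if it is a BP_Goblin.
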(event `self.ReceiveHit`
  (params (MyComp :type "PrimitiveComponent Object Reference") (Other :type "Actor Object Reference") (OtherComp :type "PrimitiveComponent Object Reference") (bSelfMoved :type Boolean) (HitLocation :type "Vector Structure") (HitNormal :type "Vector Structure") (NormalImpulse :type "Vector Structure") (Hit :type "HitResult Structure (by ref)"))
  ;[1 1 1] Check for Event Hit on Goblin
  (`self.K2_DestroyActor` Other)
  (bind _asbp_goblin (cast `/Game/Blueprint/BP_Goblin` Other))
  (`/Game/Blueprint/BP_Goblin.DamageHealth` _asbp_goblin))

(event `self.ReceiveActorBeginOverlap`
  (params (OtherActor :type "Actor Object Reference"))
  (if (`KismetSystemLibrary.DoesImplementInterface` OtherActor "/Game/Blueprint/iDamageable.iDamageable_C")
    (if (not (`self.ActorHasTag` OtherActor "Friendly"))
      (message `/Game/Blueprint/iDamageable.AffectHealth` OtherActor (`self.Damage`))
      (`GameplayStatics.SpawnSoundAttached` "/Game/sound/SC_MissileExplosion.SC_MissileExplosion" (`self.Laser mesh`) :!label _label)
      (`self.K2_DestroyActor`)
      ;[1 1 1] Damage Enemy on Contact
      (bind _asenemy_character (cast `/Game/Blueprint/NPC_AI/EnemyCharacter` OtherActor))
      (`/Game/Blueprint/NPC_AI/EnemyCharacter.DamageHealth` _asenemy_character))
    (else
      (goto _label))))

(fn `UserConstructionScript`)