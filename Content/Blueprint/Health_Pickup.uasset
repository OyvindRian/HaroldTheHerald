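; Health pickup actor for the twin-stick game that restores the player's health on overlap.
; It spins its cube every tick and destroys itself 30 seconds after spawning.
; When BP_TwinStickCharacter overlaps it below full health, it adds HealthPickupValue capped at 100 and calls the character's HealthPickup.
; It then plays a particle burst and sound before destroying itself; at full health it stays.
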(event `self.ReceiveBeginPlay`
  ;[1 1 1] Despawn after 30 seconds
  (`KismetSystemLibrary.Delay` 30.0)
  (`self.K2_DestroyActor`))

(event `self.ReceiveTick`
  (params (DeltaSeconds :type "Float (single-precision)"))
  ;[1 1 1] Rotate health cube
  (`SceneComponent.K2_AddRelativeRotation` (`self.Cube`) (struct :`Yaw` 2.0) false false))

(event `self.Health_pickup.OnComponentBeginOverlap`
  (params (OverlappedComponent :type "PrimitiveComponent Object Reference") (OtherActor :type "Actor Object Reference") (OtherComp :type "PrimitiveComponent Object Reference") (OtherBodyIndex :type Integer) (bFromSweep :type Boolean) (SweepResult :type "HitResult Structure (by ref)"))
  (bind _returnvalue (`self.K2_GetActorLocation`))
  (bind _asbp_twin_stick_character (cast `/Game/Blueprint/BP_TwinStickCharacter` OtherActor))
  (bind _healthpoint (`/Game/Blueprint/BP_TwinStickCharacter.HealthPoint` _asbp_twin_stick_character))
  ;[1 1 1] Check If Player Health is under 100
  (if (<= _healthpoint 99.0)
    (set `/Game/Blueprint/BP_TwinStickCharacter.HealthPoint` (`KismetMathLibrary.FClamp` (+ _healthpoint (`self.HealthPickupValue`)) 0.0 100.0) _asbp_twin_stick_character)
    (`/Game/Blueprint/BP_TwinStickCharacter.HealthPickup` _asbp_twin_stick_character)
    (`GameplayStatics.SpawnEmitterAtLocation` "/Game/VFX_Toolkit_V1/ParticleSystems/356Days/Par_KineticForce_01.Par_KineticForce_01" _returnvalue (struct) (0.1 0.1 0.1))
    (`GameplayStatics.SpawnSoundAtLocation` "/Game/sound/Health_Pickup_Cue.Health_Pickup_Cue" _returnvalue)
    (`self.K2_DestroyActor`)))

(fn `UserConstructionScript`)